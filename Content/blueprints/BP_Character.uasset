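; BP_Character is a character Blueprint that supports either a first-person or a third-person camera and shows a sight widget on screen.
; The construction script uses UseFirstPersonView to set auto-activation on the FPS camera, or on the TPS camera and its boom.
; On BeginPlay it creates BP_Sight and adds it to the viewport.
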(event `self.ReceiveBeginPlay`
  (bind _returnvalue (`|CreateWidget` "/Game/widgets/BP_Sight.BP_Sight_C"))
  (`UserWidget.AddToViewport` _returnvalue 0))

(fn `UserConstructionScript`
  (`ActorComponent.SetAutoActivate` (`self.FPSCameraComponent`) (`self.bUseFirstPersonView`))
  (`ActorComponent.SetAutoActivate` (`self.TPSCameraComponent`) (not (`self.bUseFirstPersonView`)))
  (`ActorComponent.SetAutoActivate` (`self.CameraBoom`) (not (`self.bUseFirstPersonView`))))